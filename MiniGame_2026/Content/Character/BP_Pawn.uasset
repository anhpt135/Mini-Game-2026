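; Pawn that changes the color of its Arm, Body and Head when struck by lightning.
; OnLightningHit lights the parts in that order on staggered delays, creating a dynamic material instance for each and raising its HitAlpha parameter.
; OnLightningStop waits briefly, then zeroes HitAlpha through nested validity checks, so a missing instance skips the remaining parts.
; Stopping does not cancel hit delays still pending.
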(event `MG26_LightningHitInterface.OnLightningHit`
  ;[0 0 0 0.5 129] LOGIC ĐỔI MÀU KHI BỊ SÉT BẮN
  ;;[0.04733 0.15 0.1419 0.5] ĐỔI MÀU ARM
  (`KismetSystemLibrary.Delay` 0.5)
  (bind _returnvalue (`PrimitiveComponent.CreateDynamicMaterialInstance` (`self.Arm`) 0 null "None"))
  (bind _output_get (set `self.DMI_Arm` _returnvalue))
  (`MaterialInstanceDynamic.SetScalarParameterValue` _output_get "HitAlpha" 1.0)
  ;;[0.15 0.01234 0.02283 0.5] ĐỔI MÀU BODY
  (`KismetSystemLibrary.Delay` 1.0)
  (bind _returnvalue_2 (`PrimitiveComponent.CreateDynamicMaterialInstance` (`self.Body`) 0 null "None"))
  (bind _output_get_2 (set `self.DMI_Body` _returnvalue_2))
  (`MaterialInstanceDynamic.SetScalarParameterValue` _output_get_2 "HitAlpha" 1.0)
  ;;[1 0.9347 0.06003 0.5] ĐỔI MÀU HEAD
  (`KismetSystemLibrary.Delay` 1.0)
  (bind _returnvalue_3 (`PrimitiveComponent.CreateDynamicMaterialInstance` (`self.Head`) 0 null "None"))
  (bind _output_get_3 (set `self.DIMI_Head` _returnvalue_3))
  (`MaterialInstanceDynamic.SetScalarParameterValue` _output_get_3 "HitAlpha" 1.0))

(event `MG26_LightningHitInterface.OnLightningStop`
  (bind _dimi_head (`self.DIMI_Head`))
  (bind _dmi_arm (`self.DMI_Arm`))
  (bind _dmi_body (`self.DMI_Body`))
  ;[0 0 0 0.5 129] LOGIC ĐỔI MÀU KHI BỊ SÉT BẮN
  ;;[0.15 0.03838 0.1313 0.5] Trả lại màu ARM
  (`KismetSystemLibrary.Delay` 0.5)
  (`/Engine/EditorBlueprintResources/StandardMacros.IsValid` _dmi_arm
    (:`Is Valid`
      (`MaterialInstanceDynamic.SetScalarParameterValue` _dmi_arm "HitAlpha" 0.0)
      ;;[0.04611 0.1249 0.15 0.5] Trả lại màu BODY
      (`/Engine/EditorBlueprintResources/StandardMacros.IsValid` _dmi_body
        (:`Is Valid`
          (`MaterialInstanceDynamic.SetScalarParameterValue` _dmi_body "HitAlpha" 0.0)
          ;;[0.02744 0.15 0.02275 0.5] Trả lại màu HEAD
          (`/Engine/EditorBlueprintResources/StandardMacros.IsValid` _dimi_head
            (:`Is Valid`
              (`MaterialInstanceDynamic.SetScalarParameterValue` _dimi_head "HitAlpha" 0.0))))))))

(fn `UserConstructionScript`)